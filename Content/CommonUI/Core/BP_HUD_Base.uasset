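; Base HUD Blueprint that owns the CommonUI layered widget stack for the owning player.
; On BeginPlay it creates WBP_CommonUI_StackLayers, stores the reference and adds it to the viewport.
; Push Widget and Remove Widget forward a stack layer and an activatable widget class or instance to that root widget, with push returning the pushed widget.
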(event EventBeginPlay
  (bind _returnvalue (UserInterface|CreateWidget "/Game/CommonUI/Widgets/StackLayers/WBP_CommonUI_StackLayers.WBP_CommonUI_StackLayers_C" (Game|Player|GetOwningPlayerController)))
  (bind _output_get (Variables|Data|SetWBP_CommonUI_StackLayers _returnvalue))
  (UserInterface|Viewport|AddtoViewport _output_get 0))

(fn ConstructionScript)

(fn PushWidget
  (params (Stack%20Layer :type E_UI_CommonUI_StackLayers%20Enum :default "NewEnumerator0") (ActivatableWidgetClass :type Common%20Activatable%20Widget%20Class%20Reference))
  (bind _common_activatable_widget (Default|PushWidget (Variables|Data|GetWBP_CommonUI_StackLayers) Stack%20Layer ActivatableWidgetClass))
  (return _common_activatable_widget))

(fn RemoveWidget
  (params (Stack%20Layer :type E_UI_CommonUI_StackLayers%20Enum :default "NewEnumerator0") (WidgetToRemove :type Common%20Activatable%20Widget%20Object%20Reference))
  (Default|RemoveWidget (Variables|Data|GetWBP_CommonUI_StackLayers) Stack%20Layer WidgetToRemove))