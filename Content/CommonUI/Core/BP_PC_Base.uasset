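; Base player controller in the CommonUI core folder that lets a gamepad input move the mouse cursor.
; The IA_Specific_GamepadCursor Enhanced Input event passes its value to SetGamepadCursorPosition, which adds it, plus a constant offset on each axis, to the current mouse position.
; The result is truncated, clamped to the viewport, printed for debugging and applied with SetMouseLocation.
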(event Input|EnhancedActionEvents|EnhancedInputActionIA_Specific_GamepadCursor
  (params (ActionValue :type Vector%202D%20Structure) (ElapsedSeconds :type Float%20%28double-precision%29) (TriggeredSeconds :type Float%20%28double-precision%29) (InputAction :type Input%20Action%20Object%20Reference :default "/Game/CommonUI/EnhancedInput/Specific/Actions/IA_Specific_GamepadCursor.IA_Specific_GamepadCursor"))
  (CallFunction|SetGamepadCursorPosition ActionValue))

(event EventBeginPlay)

(event EventTick
  (params (DeltaSeconds :type Float%20%28single-precision%29)))

(fn ConstructionScript)

(fn SetGamepadCursorPosition
  (params (Action%20Value :type Vector%202D%20Structure))
  (bind (_locationx _locationy) (Game|Player|GetMousePosition))
  (bind (_x _y) (Math|Vector2D|BreakVector2D Action%20Value))
  (bind _returnvalue (Viewport|GetViewportSize))
  (bind (_x_2 _y_2) (Math|Vector2D|BreakVector2D _returnvalue))
  (bind _returnvalue_2 (+ _y 1e+01))
  (bind _returnvalue_3 (+ _x 1e+01))
  (bind _returnvalue_4 (Math|Float|Truncate _x_2))
  (bind _returnvalue_5 (Math|Float|Truncate _y_2))
  (bind _returnvalue_6 (+ (Math|Vector2D|MakeVector2D _returnvalue_3 _returnvalue_2) (Math|Vector2D|MakeVector2D _locationx _locationy)))
  (bind (_x_3 _y_3) (Math|Vector2D|BreakVector2D _returnvalue_6))
  (bind _returnvalue_7 (Math|Float|Truncate _x_3))
  (bind _returnvalue_8 (Math|Float|Truncate _y_3))
  (bind _returnvalue_9 (Math|Integer|Clamp(Integer) _returnvalue_7 0 _returnvalue_4))
  (bind _returnvalue_10 (Math|Integer|Clamp(Integer) _returnvalue_8 0 _returnvalue_5))
  (Development|PrintString (Utilities|String|Append (Utilities|String|ToString(Integer) _returnvalue_9) " , " (Utilities|String|ToString(Integer) _returnvalue_10)))
  (Class|PlayerController|SetMouseLocation _returnvalue_9 _returnvalue_10))